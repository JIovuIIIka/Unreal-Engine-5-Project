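; Traffic light Blueprint that endlessly cycles its Green, Yellow and Red lamps on timed delays.
; BeginPlay waits RtoY, YtoG and GtoR in turn, calling TurnYellow, TurnGreen and TurnRed, then calls the Recolor event, which re-enters the chain to loop.
; Each Turn function applies that lamp's lit material and resets the other two to M_TrafficColor.
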(event Custom|Recolor
  (Utilities|FlowControl|Delay (Variables|Default|GetRtoY))
  (CallFunction|TurnYellow)
  (Utilities|FlowControl|Delay (Variables|Default|GetYtoG))
  (CallFunction|TurnGreen)
  (Utilities|FlowControl|Delay (Variables|Default|GetGtoR))
  (CallFunction|TurnRed)
  (CallFunction|Recolor))

(event EventBeginPlay
  (Utilities|FlowControl|Delay (Variables|Default|GetRtoY))
  (CallFunction|TurnYellow)
  (Utilities|FlowControl|Delay (Variables|Default|GetYtoG))
  (CallFunction|TurnGreen)
  (Utilities|FlowControl|Delay (Variables|Default|GetGtoR))
  (CallFunction|TurnRed)
  (CallFunction|Recolor))

(event Collision|EventActorBeginOverlap
  (params (OtherActor :type Actor%20Object%20Reference)))

(event EventTick
  (params (DeltaSeconds :type Float%20%28single-precision%29)))

(fn ConstructionScript)

(fn TurnGreen
  (Rendering|Material|SetMaterial (Variables|Default|GetGreen) 0 "/Game/Blueprints/Materials/GreenMaterial.GreenMaterial")
  (Rendering|Material|SetMaterial (Variables|Default|GetYellow) 0 "/Game/Blueprints/Materials/M_TrafficColor.M_TrafficColor")
  (Rendering|Material|SetMaterial (Variables|Default|GetRed) 0 "/Game/Blueprints/Materials/M_TrafficColor.M_TrafficColor"))

(fn TurnYellow
  (Rendering|Material|SetMaterial (Variables|Default|GetGreen) 0 "/Game/Blueprints/Materials/M_TrafficColor.M_TrafficColor")
  (Rendering|Material|SetMaterial (Variables|Default|GetYellow) 0 "/Game/Blueprints/Materials/YellowMaterial.YellowMaterial")
  (Rendering|Material|SetMaterial (Variables|Default|GetRed) 0 "/Game/Blueprints/Materials/M_TrafficColor.M_TrafficColor"))

(fn TurnRed
  (Rendering|Material|SetMaterial (Variables|Default|GetGreen) 0 "/Game/Blueprints/Materials/M_TrafficColor.M_TrafficColor")
  (Rendering|Material|SetMaterial (Variables|Default|GetYellow) 0 "/Game/Blueprints/Materials/M_TrafficColor.M_TrafficColor")
  (Rendering|Material|SetMaterial (Variables|Default|GetRed) 0 "/Game/Blueprints/Materials/RedMaterial.RedMaterial"))